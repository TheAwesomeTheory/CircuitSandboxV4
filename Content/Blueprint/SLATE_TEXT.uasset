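; A VR slate actor that displays five low-poly text fields and can be picked up and dropped with motion controllers.
; The construction script gives each text component its parent mesh and per-instance text and top-character values, and BeginPlay tells all five to write.
; Pickup, called by BP_MotionController, disables physics and attaches the root to the controller; Drop re-enables physics and detaches.
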(event Collision|EventActorBeginOverlap
  (params (OtherActor :type Actor%20Object%20Reference)))

(event EventTick
  (params (DeltaSeconds :type Float%20%28single-precision%29)))

(event EventPickup
  (params (AttachTo :type Scene%20Component%20Object%20Reference) (GrabbedComponent :type Scene%20Component%20Object%20Reference))
  (Physics|SetSimulatePhysics (Variables|Debug|GetStaticMeshComponent) false)
  (Transformation|AttachComponentToComponent (VehicleSound|GetRootComponent) AttachTo "None" "KeepWorld" "KeepWorld" "KeepWorld" false))

(event EventBeginPlay
  (for _array_element (Utilities|Array|MakeArray (Variables|Default|GetLowPolyTextComp4) (Variables|Default|GetLowPolyTextComp3) (Variables|Default|GetLowPolyTextComp) (Variables|Default|GetLowPolyTextComp1) (Variables|Default|GetLowPolyTextComp2))
    (Default|Write _array_element)))

(event EventDrop
  (Physics|SetSimulatePhysics (Variables|Debug|GetStaticMeshComponent) true)
  (Transformation|DetachFromActor "KeepWorld" "KeepWorld" "KeepWorld"))

(fn ConstructionScript
  (bind _lowpolytextcomp4 (Variables|Default|GetLowPolyTextComp4))
  (bind _lowpolytextcomp3 (Variables|Default|GetLowPolyTextComp3))
  (bind _lowpolytextcomp1 (Variables|Default|GetLowPolyTextComp1))
  (bind _lowpolytextcomp2 (Variables|Default|GetLowPolyTextComp2))
  (bind _lowpolytextcomp (Variables|Default|GetLowPolyTextComp))
  (Variables|/Game/Blueprint/LowPolyTextComp.LowPolyTextComp_C|SetParentMeshRef (Variables|Default|GetLowPolyTextComp) (Variables|Default|GetStaticMesh))
  (Variables|/Game/Blueprint/LowPolyTextComp.LowPolyTextComp_C|SetParentMeshRef (Variables|Default|GetLowPolyTextComp1) (Variables|Default|GetStaticMesh1))
  (Variables|/Game/Blueprint/LowPolyTextComp.LowPolyTextComp_C|SetParentMeshRef (Variables|Default|GetLowPolyTextComp2) (Variables|Default|GetStaticMesh2))
  (Variables|/Game/Blueprint/LowPolyTextComp.LowPolyTextComp_C|SetParentMeshRef (Variables|Default|GetLowPolyTextComp3) (Variables|Default|GetStaticMesh3))
  (Variables|/Game/Blueprint/LowPolyTextComp.LowPolyTextComp_C|SetParentMeshRef (Variables|Default|GetLowPolyTextComp4) (Variables|Default|GetStaticMesh4))
  (Variables|/Game/Blueprint/LowPolyTextComp.LowPolyTextComp_C|SetRenTExt _lowpolytextcomp (Variables|Default|GetNewVar_0))
  (Variables|/Game/Blueprint/LowPolyTextComp.LowPolyTextComp_C|SetCharacter%20Top _lowpolytextcomp (Variables|Default|GetNewVar_5))
  (Variables|/Game/Blueprint/LowPolyTextComp.LowPolyTextComp_C|SetRenTExt _lowpolytextcomp1 (Variables|Default|GetNewVar_1))
  (Variables|/Game/Blueprint/LowPolyTextComp.LowPolyTextComp_C|SetCharacter%20Top _lowpolytextcomp1 (Variables|Default|GetNewVar_6))
  (Variables|/Game/Blueprint/LowPolyTextComp.LowPolyTextComp_C|SetRenTExt _lowpolytextcomp2 (Variables|Default|GetNewVar_2))
  (Variables|/Game/Blueprint/LowPolyTextComp.LowPolyTextComp_C|SetCharacter%20Top _lowpolytextcomp2 (Variables|Default|GetNewVar_7))
  (Variables|/Game/Blueprint/LowPolyTextComp.LowPolyTextComp_C|SetRenTExt _lowpolytextcomp3 (Variables|Default|GetNewVar_3))
  (Variables|/Game/Blueprint/LowPolyTextComp.LowPolyTextComp_C|SetCharacter%20Top _lowpolytextcomp3 (Variables|Default|GetNewVar_8))
  (Variables|/Game/Blueprint/LowPolyTextComp.LowPolyTextComp_C|SetRenTExt _lowpolytextcomp4 (Variables|Default|GetNewVar_4))
  (Variables|/Game/Blueprint/LowPolyTextComp.LowPolyTextComp_C|SetCharacter%20Top _lowpolytextcomp4 (Variables|Default|GetNewVar_9)))
(event Custom|Write
  (Utilities|FlowControl|Delay 0.01)
  (bind _returnvalue (Game|SpawnActorfromClass "/Game/Blueprint/LowP_TextRender.LowP_TextRender_C" (Transformation|GetWorldTransform (Variables|Default|GetParentMeshRef)) "AlwaysSpawn" 0 (Variables|Default|GetRenTExt) (Variables|Default|GetCharacter%20Top) (Variables|Default|GetChar%20Material)))
  (bind _output_get (Variables|Default|SetLetter%20LP%20Text%20REnder _returnvalue))
  (Utilities|FlowControl|Sequence
    (:then_0
      (Utilities|IsValid _output_get
        (:Is%20Valid
          (Development|PrintString "I HAs Spawned"))
        (:Is%20Not%20Valid
          (Development|PrintString "WON't SPAWN"))))
    (:then_1
      (Transformation|AttachActorToActor _output_get (Components|GetOwner) "None" "KeepWorld" "KeepWorld" "KeepWorld" true))))

(event Custom|Erase
  (Default|EraseText (Variables|Default|GetLetter%20LP%20Text%20REnder)))

(event Custom|Destroy%20TExt
  (Actor|DestroyActor (Variables|Default|GetLetter%20LP%20Text%20REnder)))
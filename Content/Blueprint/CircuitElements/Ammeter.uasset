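; Ammeter circuit element that motion controllers can pick up and drop, showing the current through it as rendered text.
; Two sphere terminals each snap one uncoupled CableCaps on overlap and release it with a pop sound when it leaves.
; PassCurrent stores the current and relays it to the opposite cap, with a retriggerable delay zeroing the reading once signals stop.
; Tick rewrites the readout on a throttled timer; the overload explosion logic is never run.
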(event OnComponentBeginOverlap(Sphere)
  (params (OverlappedComponent :type Primitive%20Component%20Object%20Reference) (OtherActor :type Actor%20Object%20Reference) (OtherComp :type Primitive%20Component%20Object%20Reference) (OtherBodyIndex :type Integer) (bFromSweep :type Boolean) (SweepResult :type Hit%20Result%20Structure%20%28by%20ref%29))
  (bind _sphere (Variables|Default|GetSphere))
  (bind _ascable_caps (Utilities|Casting|CastToCableCaps OtherActor))
  (if (and (!= _ascable_caps (Variables|Default|GetNewVar_1)) (!= _ascable_caps (Variables|Default|GetNewVar_0)))
    (if (not (Variables|/Game/Blueprint/CircuitElements/CableCaps.CableCaps_C|GetCoupled? _ascable_caps))
      (if (not (Variables|Default|GetCON%201))
        (Variables|Default|SetCON%201 true)
        (Default|Connectto _ascable_caps (Transformation|GetWorldRotation _sphere) (Transformation|GetWorldLocation _sphere) self)
        (Variables|Default|SetNewVar_0 _ascable_caps)))))

(event OnComponentBeginOverlap(Sphere1)
  (params (OverlappedComponent :type Primitive%20Component%20Object%20Reference) (OtherActor :type Actor%20Object%20Reference) (OtherComp :type Primitive%20Component%20Object%20Reference) (OtherBodyIndex :type Integer) (bFromSweep :type Boolean) (SweepResult :type Hit%20Result%20Structure%20%28by%20ref%29))
  (bind _sphere1 (Variables|Default|GetSphere1))
  (bind _ascable_caps (Utilities|Casting|CastToCableCaps OtherActor))
  (if (!= _ascable_caps (Variables|Default|GetNewVar_0))
    (if (not (Variables|/Game/Blueprint/CircuitElements/CableCaps.CableCaps_C|GetCoupled? _ascable_caps))
      (if (not (Variables|Default|GetCON%202))
        (Variables|Default|SetCON%202 true)
        (Default|Connectto _ascable_caps (Transformation|GetWorldRotation _sphere1) (Transformation|GetWorldLocation _sphere1) self)
        (Variables|Default|SetNewVar_1 _ascable_caps)))))

(event OnComponentEndOverlap(Sphere)
  (params (OverlappedComponent :type Primitive%20Component%20Object%20Reference) (OtherActor :type Actor%20Object%20Reference) (OtherComp :type Primitive%20Component%20Object%20Reference) (OtherBodyIndex :type Integer))
  (bind _ascable_caps (Utilities|Casting|CastToCableCaps OtherActor))
  (if (== OtherActor (Variables|Default|GetNewVar_0))
    (Variables|/Game/Blueprint/CircuitElements/CableCaps.CableCaps_C|SetCoupled? _ascable_caps false)
    (Variables|Default|SetCON%201 false)
    (Variables|/Game/Blueprint/CircuitElements/CableCaps.CableCaps_C|SetOwning%20Actor (Variables|Default|GetNewVar_0) 0)
    (Variables|Default|SetNewVar_0 0)
    (Audio|PlaySoundatLocation "/Game/Audio/cartoonpop.cartoonpop" (Transformation|GetActorLocation))))

(event OnComponentEndOverlap(Sphere1)
  (params (OverlappedComponent :type Primitive%20Component%20Object%20Reference) (OtherActor :type Actor%20Object%20Reference) (OtherComp :type Primitive%20Component%20Object%20Reference) (OtherBodyIndex :type Integer))
  (bind _ascable_caps (Utilities|Casting|CastToCableCaps OtherActor))
  (if (== OtherActor (Variables|Default|GetNewVar_1))
    (Variables|/Game/Blueprint/CircuitElements/CableCaps.CableCaps_C|SetCoupled? _ascable_caps false)
    (Variables|Default|SetCON%202 false)
    (Variables|/Game/Blueprint/CircuitElements/CableCaps.CableCaps_C|SetOwning%20Actor (Variables|Default|GetNewVar_1) 0)
    (Variables|Default|SetNewVar_1 0)
    (Audio|PlaySoundatLocation "/Game/Audio/cartoonpop.cartoonpop" (Transformation|GetActorLocation))))

(event EventBeginPlay
  (Default|Write (Variables|Default|GetAMpsLiteral)))

(event EventPassCurrent
  (params (Current :type Float%20%28single-precision%29) (Resistance :type Float%20%28single-precision%29) (Closed%20Circuit :type Boolean) (Passer :type Object%20Object%20Reference) (Nodal%20Current :type Float%20%28single-precision%29) (Nodal%20Resistance :type Float%20%28single-precision%29) (Node%20Mode :type NodeEnum%20Enum :default "NewEnumerator0"))
  (Utilities|FlowControl|Sequence
    (:then_0
      (Utilities|FlowControl|RetriggerableDelay 0.1)
      (Variables|Default|SetCurrent 0.0))
    (:then_1
      (if (== Passer (Variables|Default|GetNewVar_0))
        (Class|PassCurrent|PassCurrent(Message) (Variables|Default|GetNewVar_1) (stale _output_get) Resistance Closed%20Circuit 0 Nodal%20Current Nodal%20Resistance Node%20Mode)
        (else
          (Class|PassCurrent|PassCurrent(Message) (Variables|Default|GetNewVar_0) (stale _output_get) Resistance Closed%20Circuit 0 Nodal%20Current Nodal%20Resistance Node%20Mode))))
    (:then_2
      (bind _output_get (Variables|Default|SetCurrent Current)))))

(event EventTick
  (params (DeltaSeconds :type Float%20%28single-precision%29))
  (bind _numamps (Variables|Default|GetNumAMps))
  (if (Variables|Default|GetUpdate%20Current)
    (Variables|Default|SetUpdate%20Current false)
    (Default|DestroyTExt _numamps)
    (Variables|/Game/Blueprint/LowPolyTextComp.LowPolyTextComp_C|SetRenTExt _numamps (Utilities|String|ToString(Text) (Utilities|Text|ToText(Float) (Variables|Default|GetCurrent) "HalfToEven" true 1 324 0 1)))
    (Default|Write _numamps)
    (Utilities|FlowControl|Delay 3.0)
    (Variables|Default|SetUpdate%20Current true)))

(event EventPickup
  (params (AttachTo :type Scene%20Component%20Object%20Reference) (GrabbedComponent :type Scene%20Component%20Object%20Reference))
  (Physics|SetSimulatePhysics (Variables|Debug|GetStaticMeshComponent) false)
  (Transformation|AttachComponentToComponent (VehicleSound|GetRootComponent) AttachTo "None" "KeepWorld" "KeepWorld" "KeepWorld" false))

(event EventDrop
  (Physics|SetSimulatePhysics (Variables|Debug|GetStaticMeshComponent) true)
  (Transformation|DetachFromActor "KeepWorld" "KeepWorld" "KeepWorld"))

(fn ConstructionScript
  (Variables|/Game/Blueprint/LowPolyTextComp.LowPolyTextComp_C|SetParentMeshRef (Variables|Default|GetNumAMps) (Variables|Default|GetAmpTextParent))
  (Variables|/Game/Blueprint/LowPolyTextComp.LowPolyTextComp_C|SetParentMeshRef (Variables|Default|GetAMpsLiteral) (Variables|Default|GetUnitsTextParent)))
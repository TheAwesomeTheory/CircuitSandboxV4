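; Light bulb circuit element for a VR electronics game, which can be picked up and dropped by the motion controller.
; Two sphere sockets snap and attach uncoupled CableCaps, releasing them when overlap ends.
; PassCurrent forwards current to the opposite cap with summed resistance, and a retriggerable delay zeroes the stored current once passing stops.
; Over-threshold explosion logic with destructible, particles and sound exists but is disconnected, so it never runs.
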(event OnComponentBeginOverlap(Sphere)
  (params (OverlappedComponent :type Primitive%20Component%20Object%20Reference) (OtherActor :type Actor%20Object%20Reference) (OtherComp :type Primitive%20Component%20Object%20Reference) (OtherBodyIndex :type Integer) (bFromSweep :type Boolean) (SweepResult :type Hit%20Result%20Structure%20%28by%20ref%29))
  (bind _sphere (Variables|Default|GetSphere))
  (bind _ascable_caps (Utilities|Casting|CastToCableCaps OtherActor))
  (if (not (Variables|/Game/Blueprint/CircuitElements/CableCaps.CableCaps_C|GetCoupled? _ascable_caps))
    (if (not (Variables|Default|GetCON%201))
      (Variables|/Game/Blueprint/CircuitElements/CableCaps.CableCaps_C|SetCoupled? _ascable_caps true)
      (Variables|Default|SetCON%201 true)
      (bind _output_get (Variables|Default|SetNewVar_0 _ascable_caps))
      (Physics|SetSimulatePhysics (Variables|/Script/Engine.StaticMeshActor|GetStaticMeshComponent _ascable_caps) false)
      (Transformation|SetActorLocation _ascable_caps (Transformation|GetWorldLocation _sphere) false false)
      (Transformation|SetActorRotation _ascable_caps (Transformation|GetWorldRotation _sphere))
      (Transformation|AttachActorToActor _ascable_caps self "None" "KeepWorld" "KeepWorld" "KeepWorld" true)
      (Development|PrintString "0")
      (Variables|/Game/Blueprint/CircuitElements/CableCaps.CableCaps_C|SetOwning%20Actor _output_get self)
      (Audio|PlaySoundatLocation "/Game/Audio/snap_togther.snap_togther" (Transformation|GetActorLocation)))))

(event OnComponentBeginOverlap(Sphere1)
  (params (OverlappedComponent :type Primitive%20Component%20Object%20Reference) (OtherActor :type Actor%20Object%20Reference) (OtherComp :type Primitive%20Component%20Object%20Reference) (OtherBodyIndex :type Integer) (bFromSweep :type Boolean) (SweepResult :type Hit%20Result%20Structure%20%28by%20ref%29))
  (bind _sphere1 (Variables|Default|GetSphere1))
  (bind _ascable_caps (Utilities|Casting|CastToCableCaps OtherActor))
  (if (not (Variables|/Game/Blueprint/CircuitElements/CableCaps.CableCaps_C|GetCoupled? _ascable_caps))
    (if (not (Variables|Default|GetCON%202))
      (Variables|/Game/Blueprint/CircuitElements/CableCaps.CableCaps_C|SetCoupled? _ascable_caps true)
      (Variables|Default|SetCON%202 true)
      (bind _output_get (Variables|Default|SetNewVar_1 _ascable_caps))
      (Physics|SetSimulatePhysics (Variables|/Script/Engine.StaticMeshActor|GetStaticMeshComponent _ascable_caps) false)
      (Transformation|SetActorLocation _ascable_caps (Transformation|GetWorldLocation _sphere1) false false)
      (Transformation|SetActorRotation _ascable_caps (Transformation|GetWorldRotation _sphere1))
      (Transformation|AttachActorToActor _ascable_caps self "None" "KeepWorld" "KeepWorld" "KeepWorld" true)
      (Development|PrintString "1")
      (Variables|/Game/Blueprint/CircuitElements/CableCaps.CableCaps_C|SetOwning%20Actor _output_get self)
      (Audio|PlaySoundatLocation "/Game/Audio/snap_togther.snap_togther" (Transformation|GetActorLocation)))))

(event OnComponentEndOverlap(Sphere)
  (params (OverlappedComponent :type Primitive%20Component%20Object%20Reference) (OtherActor :type Actor%20Object%20Reference) (OtherComp :type Primitive%20Component%20Object%20Reference) (OtherBodyIndex :type Integer))
  (bind _ascable_caps (Utilities|Casting|CastToCableCaps OtherActor))
  (if (== OtherActor (Variables|Default|GetNewVar_0))
    (Variables|/Game/Blueprint/CircuitElements/CableCaps.CableCaps_C|SetCoupled? _ascable_caps false)
    (Variables|Default|SetCON%201 false)
    (Variables|/Game/Blueprint/CircuitElements/CableCaps.CableCaps_C|SetOwning%20Actor (stale OnComponentBeginOverlap(Sphere) _output_get) 0)
    (Variables|Default|SetNewVar_0 0)
    (Audio|PlaySoundatLocation "/Game/Audio/cartoonpop.cartoonpop" (Transformation|GetActorLocation))))

(event OnComponentEndOverlap(Sphere1)
  (params (OverlappedComponent :type Primitive%20Component%20Object%20Reference) (OtherActor :type Actor%20Object%20Reference) (OtherComp :type Primitive%20Component%20Object%20Reference) (OtherBodyIndex :type Integer))
  (bind _ascable_caps (Utilities|Casting|CastToCableCaps OtherActor))
  (if (== OtherActor (Variables|Default|GetNewVar_1))
    (Variables|/Game/Blueprint/CircuitElements/CableCaps.CableCaps_C|SetCoupled? _ascable_caps false)
    (Variables|Default|SetCON%202 false)
    (Variables|/Game/Blueprint/CircuitElements/CableCaps.CableCaps_C|SetOwning%20Actor (stale OnComponentBeginOverlap(Sphere1) _output_get) 0)
    (Variables|Default|SetNewVar_1 0)
    (Audio|PlaySoundatLocation "/Game/Audio/cartoonpop.cartoonpop" (Transformation|GetActorLocation))))

(event Custom|Pass%20Current
  (params (current :type Float%20%28single-precision%29) (resistance :type Integer) (ClosedCircuit :type Boolean) (Passer :type Object%20Object%20Reference))
  (bind _returnvalue (+ (Variables|Default|Getresistance) resistance))
  (Utilities|FlowControl|Sequence
    (:then_0
      (if (== Passer (Variables|Default|GetNewVar_0))
        (Default|PassCurrentFirstCap (Variables|Default|GetNewVar_1) current _returnvalue ClosedCircuit)
        (else
          (Default|PassCurrentFirstCap (Variables|Default|GetNewVar_0) current _returnvalue ClosedCircuit))))
    (:then_1
      (Variables|Default|SetCurrent current))
    (:then_2
      (Utilities|FlowControl|RetriggerableDelay 0.1)
      (Variables|Default|SetCurrent 0.0))))

(event EventBeginPlay)

(event Collision|EventActorBeginOverlap
  (params (OtherActor :type Actor%20Object%20Reference)))

(event EventTick
  (params (DeltaSeconds :type Float%20%28single-precision%29))
  (if (Variables|Default|GetExploded?)
    _))

(event EventPickup
  (params (AttachTo :type Scene%20Component%20Object%20Reference) (GrabbedComponent :type Scene%20Component%20Object%20Reference))
  (Physics|SetSimulatePhysics (Variables|Debug|GetStaticMeshComponent) false)
  (Transformation|AttachComponentToComponent (VehicleSound|GetRootComponent) AttachTo "None" "KeepWorld" "KeepWorld" "KeepWorld" false))

(event EventDrop
  (Physics|SetSimulatePhysics (Variables|Debug|GetStaticMeshComponent) true)
  (Transformation|DetachFromActor "KeepWorld" "KeepWorld" "KeepWorld"))

(fn ConstructionScript)
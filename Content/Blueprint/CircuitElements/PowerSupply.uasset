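; VR power supply for a circuit-building game, which can be picked up and has motion-controller buttons to adjust its displayed voltage within limits.
; Two sphere terminals snap and attach CableCaps on overlap, releasing them and opening the circuit on end overlap.
; Tick feeds current into the first terminal's cap.
; CircuitClosed derives current from voltage over equivalent resistance, and its retriggerable delay reopens the circuit unless the event keeps firing.
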(event OnComponentBeginOverlap(Sphere)
  (params (OverlappedComponent :type Primitive%20Component%20Object%20Reference) (OtherActor :type Actor%20Object%20Reference) (OtherComp :type Primitive%20Component%20Object%20Reference) (OtherBodyIndex :type Integer) (bFromSweep :type Boolean) (SweepResult :type Hit%20Result%20Structure%20%28by%20ref%29))
  (bind _sphere (Variables|Default|GetSphere))
  (bind _ascable_caps (Utilities|Casting|CastToCableCaps OtherActor))
  (if (not (Variables|/Game/Blueprint/CircuitElements/CableCaps.CableCaps_C|GetCoupled? _ascable_caps))
    (if (not (Variables|Default|GetCON%201))
      (Variables|/Game/Blueprint/CircuitElements/CableCaps.CableCaps_C|SetCoupled? _ascable_caps true)
      (Variables|Default|SetCON%201 true)
      (bind _output_get (Variables|Default|SetNewVar_0 _ascable_caps))
      (Physics|SetSimulatePhysics (Variables|/Script/Engine.StaticMeshActor|GetStaticMeshComponent _ascable_caps) false)
      (Transformation|SetActorLocation _ascable_caps (Transformation|GetWorldLocation _sphere) false false)
      (Transformation|SetActorRotation _ascable_caps (Transformation|GetWorldRotation _sphere))
      (Transformation|AttachActorToActor _ascable_caps self "None" "KeepWorld" "KeepWorld" "KeepWorld" true)
      (Variables|/Game/Blueprint/CircuitElements/CableCaps.CableCaps_C|SetOwning%20Actor _output_get self)
      (Audio|PlaySoundatLocation "/Game/Audio/snap_togther.snap_togther" (Transformation|GetActorLocation)))))

(event OnComponentBeginOverlap(Sphere1)
  (params (OverlappedComponent :type Primitive%20Component%20Object%20Reference) (OtherActor :type Actor%20Object%20Reference) (OtherComp :type Primitive%20Component%20Object%20Reference) (OtherBodyIndex :type Integer) (bFromSweep :type Boolean) (SweepResult :type Hit%20Result%20Structure%20%28by%20ref%29))
  (bind _sphere1 (Variables|Default|GetSphere1))
  (bind _ascable_caps (Utilities|Casting|CastToCableCaps OtherActor))
  (if (not (Variables|/Game/Blueprint/CircuitElements/CableCaps.CableCaps_C|GetCoupled? _ascable_caps))
    (if (not (Variables|Default|GetCON%202))
      (Variables|/Game/Blueprint/CircuitElements/CableCaps.CableCaps_C|SetCoupled? _ascable_caps true)
      (Variables|Default|SetCON%202 true)
      (bind _output_get (Variables|Default|SetNewVar_1 _ascable_caps))
      (Physics|SetSimulatePhysics (Variables|/Script/Engine.StaticMeshActor|GetStaticMeshComponent _ascable_caps) false)
      (Transformation|SetActorLocation _ascable_caps (Transformation|GetWorldLocation _sphere1) false false)
      (Transformation|SetActorRotation _ascable_caps (Transformation|GetWorldRotation _sphere1))
      (Transformation|AttachActorToActor _ascable_caps self "None" "KeepWorld" "KeepWorld" "KeepWorld" true)
      (Variables|/Game/Blueprint/CircuitElements/CableCaps.CableCaps_C|SetOwning%20Actor _output_get self)
      (Audio|PlaySoundatLocation "/Game/Audio/snap_togther.snap_togther" (Transformation|GetActorLocation)))))

(event OnComponentEndOverlap(Sphere)
  (params (OverlappedComponent :type Primitive%20Component%20Object%20Reference) (OtherActor :type Actor%20Object%20Reference) (OtherComp :type Primitive%20Component%20Object%20Reference) (OtherBodyIndex :type Integer))
  (bind _ascable_caps (Utilities|Casting|CastToCableCaps OtherActor))
  (if (== OtherActor (Variables|Default|GetNewVar_0))
    (Variables|/Game/Blueprint/CircuitElements/CableCaps.CableCaps_C|SetCoupled? _ascable_caps false)
    (Variables|Default|SetCON%201 false)
    (Variables|/Game/Blueprint/CircuitElements/CableCaps.CableCaps_C|SetOwning%20Actor (stale OnComponentBeginOverlap(Sphere) _output_get) 0)
    (CallFunction|CircuitOpen)
    (Variables|Default|SetNewVar_0 0)
    (Audio|PlaySoundatLocation "/Game/Audio/cartoonpop.cartoonpop" (Transformation|GetActorLocation))))

(event OnComponentEndOverlap(Sphere1)
  (params (OverlappedComponent :type Primitive%20Component%20Object%20Reference) (OtherActor :type Actor%20Object%20Reference) (OtherComp :type Primitive%20Component%20Object%20Reference) (OtherBodyIndex :type Integer))
  (bind _ascable_caps (Utilities|Casting|CastToCableCaps OtherActor))
  (if (== OtherActor (Variables|Default|GetNewVar_1))
    (Variables|/Game/Blueprint/CircuitElements/CableCaps.CableCaps_C|SetCoupled? _ascable_caps false)
    (Variables|Default|SetCON%202 false)
    (Variables|/Game/Blueprint/CircuitElements/CableCaps.CableCaps_C|SetOwning%20Actor (stale OnComponentBeginOverlap(Sphere1) _output_get) 0)
    (CallFunction|CircuitOpen)
    (Variables|Default|SetNewVar_1 0)
    (Audio|PlaySoundatLocation "/Game/Audio/cartoonpop.cartoonpop" (Transformation|GetActorLocation))))

(event OnComponentBeginOverlap(UpButCol)
  (params (OverlappedComponent :type Primitive%20Component%20Object%20Reference) (OtherActor :type Actor%20Object%20Reference) (OtherComp :type Primitive%20Component%20Object%20Reference) (OtherBodyIndex :type Integer) (bFromSweep :type Boolean) (SweepResult :type Hit%20Result%20Structure%20%28by%20ref%29))
  (bind _lowpolytextvoltage (Variables|Default|GetLowPolyTextVoltage))
  ;[1 1 1] Up Button
  (Utilities|Casting|CastToBP_MotionController OtherActor)
  (if (< (Variables|Default|GetVoltage) (Variables|Default|GetVoltage%20upper%20limit))
    (Math|Integer|IncrementInt (Variables|Default|GetVoltage)
      (:%20%20
        (Default|DestroyTExt _lowpolytextvoltage)
        (Variables|/Game/Blueprint/LowPolyTextComp.LowPolyTextComp_C|SetRenTExt _lowpolytextvoltage (Utilities|String|BuildString(Integer) "" "" (Variables|Default|GetVoltage) " V"))
        (Default|Write _lowpolytextvoltage)
        (Audio|PlaySoundatLocation "/Game/Audio/clickupdown.clickupdown" (Transformation|GetActorLocation))
        (Rendering|Material|SetMaterial (Variables|Default|GetUPBUT) 0 "/Game/Materials/Master_Emissive_White.Master_Emissive_White")))))

(event OnComponentEndOverlap(UpButCol)
  (params (OverlappedComponent :type Primitive%20Component%20Object%20Reference) (OtherActor :type Actor%20Object%20Reference) (OtherComp :type Primitive%20Component%20Object%20Reference) (OtherBodyIndex :type Integer))
  (Rendering|Material|SetMaterial (Variables|Default|GetUPBUT) 0 "/Game/StarterContent/Materials/M_Basic_Wall.M_Basic_Wall"))

(event OnComponentEndOverlap(DownButCol)
  (params (OverlappedComponent :type Primitive%20Component%20Object%20Reference) (OtherActor :type Actor%20Object%20Reference) (OtherComp :type Primitive%20Component%20Object%20Reference) (OtherBodyIndex :type Integer))
  (Rendering|Material|SetMaterial (Variables|Default|GetDownBut) 0 "/Game/StarterContent/Materials/M_Basic_Wall.M_Basic_Wall"))

(event OnComponentBeginOverlap(DownButCol)
  (params (OverlappedComponent :type Primitive%20Component%20Object%20Reference) (OtherActor :type Actor%20Object%20Reference) (OtherComp :type Primitive%20Component%20Object%20Reference) (OtherBodyIndex :type Integer) (bFromSweep :type Boolean) (SweepResult :type Hit%20Result%20Structure%20%28by%20ref%29))
  (bind _lowpolytextvoltage (Variables|Default|GetLowPolyTextVoltage))
  ;[1 1 1] Down Button
  (Utilities|Casting|CastToBP_MotionController OtherActor)
  (if (> (Variables|Default|GetVoltage) (Variables|Default|GetVoltage%20lower%20limit))
    (Math|Integer|DecrementInt (Variables|Default|GetVoltage)
      (:%20%20
        (Default|DestroyTExt _lowpolytextvoltage)
        (Variables|/Game/Blueprint/LowPolyTextComp.LowPolyTextComp_C|SetRenTExt _lowpolytextvoltage (Utilities|String|BuildString(Integer) "" "" (Variables|Default|GetVoltage) " V"))
        (Default|Write _lowpolytextvoltage)
        (Audio|PlaySoundatLocation "/Game/Audio/clickupdown.clickupdown" (Transformation|GetActorLocation))
        (Rendering|Material|SetMaterial (Variables|Default|GetDownBut) 0 "/Game/Materials/Emissive_Simple.Emissive_Simple")))))

(event Custom|Circuit%20Closed
  (params (Equivalent%20Resistance :type Integer))
  (Variables|Default|SetEQ%20Resist Equivalent%20Resistance)
  (Variables|Default|SetCircuitClosed true)
  (Variables|Default|SetCurrent (/ (Math|Conversions|ToFloat(Integer) (Variables|Default|GetVoltage)) (Math|Conversions|ToFloat(Integer) (Variables|Default|GetEQ%20Resist))))
  (Utilities|FlowControl|RetriggerableDelay 0.1)
  (CallFunction|CircuitOpen))

(event Custom|Circuit%20Open
  (Variables|Default|SetEQ%20Resist 0)
  (Variables|Default|SetCircuitClosed false)
  (Variables|Default|SetCurrent 0.0))

(event EventBeginPlay
  (bind _lowpolytextvoltage (Variables|Default|GetLowPolyTextVoltage))
  (Default|Write (Variables|Default|GetLowPolyTextPos))
  (Default|Write (Variables|Default|GetLowPolyTextNeg))
  (Variables|/Game/Blueprint/LowPolyTextComp.LowPolyTextComp_C|SetRenTExt _lowpolytextvoltage (Utilities|String|BuildString(Integer) "" "" (Variables|Default|GetVoltage) " V"))
  (Default|Write _lowpolytextvoltage))

(event EventTick
  (params (DeltaSeconds :type Float%20%28single-precision%29))
  (if (Utilities|IsValid (Variables|Default|GetNewVar_0))
    (if (Variables|Default|GetCircuitClosed)
      (Default|PassCurrentFirstCap (Variables|Default|GetNewVar_0) (Variables|Default|GetCurrent) 0 false)
      (else
        (Default|PassCurrentFirstCap (Variables|Default|GetNewVar_0) 0.0 0 false)
        (Default|PassCurrentFirstCap (Variables|Default|GetNewVar_1) 0.0 0 false)))))

(event EventPickup
  (params (AttachTo :type Scene%20Component%20Object%20Reference) (GrabbedComponent :type Scene%20Component%20Object%20Reference))
  (Physics|SetSimulatePhysics (Variables|Debug|GetStaticMeshComponent) false)
  (Transformation|AttachComponentToComponent (VehicleSound|GetRootComponent) AttachTo "None" "KeepWorld" "KeepWorld" "KeepWorld" false))

(event EventDrop
  (Physics|SetSimulatePhysics (Variables|Debug|GetStaticMeshComponent) true)
  (Transformation|DetachFromActor "KeepWorld" "KeepWorld" "KeepWorld"))

(fn ConstructionScript
  (Variables|/Game/Blueprint/LowPolyTextComp.LowPolyTextComp_C|SetParentMeshRef (Variables|Default|GetLowPolyTextPos) (Variables|Default|GetTPPos))
  (Variables|/Game/Blueprint/LowPolyTextComp.LowPolyTextComp_C|SetParentMeshRef (Variables|Default|GetLowPolyTextNeg) (Variables|Default|GetTPNEG))
  (Variables|/Game/Blueprint/LowPolyTextComp.LowPolyTextComp_C|SetParentMeshRef (Variables|Default|GetLowPolyTextVoltage) (Variables|Default|GetTPVoltage)))
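; LowP_TextRender is an actor Blueprint that renders a string as 3D text built from static mesh letters.
; The construction script calls GenerateText, which adds one mesh component per character, spaced along X by CharaterGap.
; GetLetter looks up each character in Alphabet for mesh, offset, rotation, scale and material, with CharacterMaterial as the fallback.
; Components are tracked in LetterArray so EraseText can destroy them; generation also prints a debug "Hello".
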(event Custom|Generate%20Text
  ;[1 1 1] Generate Text
  (for _index (range 0 (Utilities|String|Len (Variables|Default|GetRenderString)))
    (bind (_mesh _newparam _newparam2 _newparam3 _materials) (Utilities|GetLetter _index)
      (:out
        (Development|PrintString "Hello")
        (bind _returnvalue (AddComponent|AddStaticMeshComponent false (Math|Transform|MakeTransform (+ _newparam (Math|Vector|MakeVector (* _index (Variables|Default|GetCharaterGap)) 0.0 0.0)) _newparam2 (|Scale _newparam3))))
        (Utilities|Array|Add (Variables|Default|GetLetter%20Array) _returnvalue)
        (Components|StaticMesh|SetStaticMesh _returnvalue _mesh)
        (if (Utilities|IsValid _materials)
          (Rendering|Material|SetMaterial _returnvalue 0 _materials)
          (else
            (Rendering|Material|SetMaterial _returnvalue 0 (Variables|Default|GetCharacter%20Material))))))))

(event Custom|Erase%20Text
  (bind _letter_array (Variables|Default|GetLetter%20Array))
  ;[1 1 1] Generate Text
  (for _array_element _letter_array
    (Components|DestroyComponent _array_element))
  (Utilities|Array|Clear _letter_array))

(event EventBeginPlay)

(event Collision|EventActorBeginOverlap
  (params (OtherActor :type Actor%20Object%20Reference)))

(event EventTick
  (params (DeltaSeconds :type Float%20%28single-precision%29)))

(fn ConstructionScript
  (CallFunction|GenerateText))